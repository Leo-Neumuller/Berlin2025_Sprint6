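; Player component that equips a BP_FPSPlayer with a portal gun and fires the first or second portal from the two interact inputs.
; On BeginPlay it spawns BP_PortalGunAttached on the first-person mesh's socket.
; Each input plays the shoot montage, whose notify triggers a trace from the gun socket toward the camera's aim.
; The gun's SendPortal receives the normal-offset impact point and hit actor's rotation, or the trace end on a miss.
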(event Input|EnhancedActionEvents|EnhancedInputActionIA_Player_Interact
  (params (ActionValue :type Boolean) (ElapsedSeconds :type Float%20%28double-precision%29) (TriggeredSeconds :type Float%20%28double-precision%29) (InputAction :type Input%20Action%20Object%20Reference :default "/Game/00-Blueprints/Inputs/Actions/IA_Player_Interact.IA_Player_Interact"))
  (:Started
    (Utilities|PlayPortalAnim true
      (:On%20Notify%20Begin
        (Utilities|PortalLogic false)))))

(event Input|EnhancedActionEvents|EnhancedInputActionIA_Player_InteractSecond
  (params (ActionValue :type Boolean) (ElapsedSeconds :type Float%20%28double-precision%29) (TriggeredSeconds :type Float%20%28double-precision%29) (InputAction :type Input%20Action%20Object%20Reference :default "/Game/00-Blueprints/Inputs/Actions/IA_Player_InteractSecond.IA_Player_InteractSecond"))
  (:Started
    (Utilities|PlayPortalAnim false
      (:On%20Notify%20Begin
        (Utilities|PortalLogic true)))))

(event EventBeginPlay
  (bind _returnvalue (Game|SpawnActorfromClass "/Game/00-Blueprints/Items/PortalGun/BP_PortalGunAttached.BP_PortalGunAttached_C" (Math|Transform|MakeTransform "0, 0, 0") "Undefined" "MultiplyWithRoot" 0 0))
  (Variables|Default|SetPortalGunRef _returnvalue)
  (bind _asbp_fpsplayer (Utilities|Casting|CastToBP_FPSPlayer (Components|GetOwner)))
  (Variables|Default|SetPlayerRef _asbp_fpsplayer)
  (Transformation|AttachComponentToComponent (Variables|Default|GetPortalGunRef) (Variables|/Game/00-Blueprints/Player/BP_FPSPlayer.BP_FPSPlayer_C|GetFirstPersonMesh _asbp_fpsplayer) "PortalGun" "SnapToTarget" "SnapToTarget" "SnapToTarget" true)
  (Variables|/Game/00-Blueprints/Player/BP_FPSPlayer.BP_FPSPlayer_C|SetIsHoldingPortalGun _asbp_fpsplayer true))