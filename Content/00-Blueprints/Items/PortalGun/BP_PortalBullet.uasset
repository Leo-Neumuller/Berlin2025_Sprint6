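; Projectile fired for the portal gun that places one of two portals when it hits a surface.
; On overlapping an actor tagged PortalSurface, it passes its stored location, rotation and first/second flag to the Portal reference's PlacePortal.
; Any other overlap spawns one of two Niagara effects chosen by that flag, and either hit destroys the bullet.
; The construction script applies its material, and a timed delay destroys stray bullets.
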(event OnComponentBeginOverlap(Sphere1)
  (params (OverlappedComponent :type Primitive%20Component%20Object%20Reference) (OtherActor :type Actor%20Object%20Reference) (OtherComp :type Primitive%20Component%20Object%20Reference) (OtherBodyIndex :type Integer) (bFromSweep :type Boolean) (SweepResult :type Hit%20Result%20Structure%20%28by%20ref%29))
  (if (Actor|ActorHasTag OtherActor "PortalSurface")
    (Default|PlacePortal (Variables|Default|GetPortal) (Variables|Default|GetFirst/Second) (Variables|Default|GetPortalLocation) (Variables|Default|GetPortalRotation))
    (Actor|DestroyActor)
    (else
      (Niagara|SpawnSystematLocation (select (Variables|Default|GetFirst/Second) (Variables|Default|GetNiagara2) (Variables|Default|GetNiagara1)) (Transformation|GetActorLocation) (Class|KismetMathLibrary|NegateRotator (Transformation|GetActorRotation)))
      (Actor|DestroyActor))))

(event EventBeginPlay
  (Utilities|FlowControl|Delay 1e+01)
  (Actor|DestroyActor))

(event Collision|EventActorBeginOverlap
  (params (OtherActor :type Actor%20Object%20Reference)))

(event EventTick
  (params (DeltaSeconds :type Float%20%28single-precision%29)))

(fn ConstructionScript
  (Rendering|Material|SetMaterial (Variables|Default|GetSphere) 0 (Variables|Default|GetMaterial)))