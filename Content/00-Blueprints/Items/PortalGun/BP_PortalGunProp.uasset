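; BP_PortalGunProp is the world pickup for the portal gun, shown with coloured lights and rotating crystals.
; On BeginPlay it tints its two point lights green and blue and starts a timeline that rotates the Crystals component in pitch.
; On Interact it adds a BP_PortalGunComponent to the interacting actor, then destroys itself.
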(event EventBeginPlay
  (|CallParentFunction)
  (Rendering|Components|Light|SetLightColor (Variables|Default|GetPointLight1) "(R=0.176471,G=1.000000,B=0.223529,A=1.000000)" true)
  (Rendering|Components|Light|SetLightColor (Variables|Default|GetPointLight) "(R=0.105882,G=0.454902,B=1.000000,A=1.000000)" true)
  (bind _newtrack_0 (Timeline|RotateCrystals Play)
    (:Update
      (Transformation|SetRelativeRotation (Variables|Default|GetCrystals) (Math|Rotator|MakeRotator 0.0 _newtrack_0 0.0) false false))))

(event EventInteract
  (params (From :type Actor%20Object%20Reference))
  (Game|AddComponentbyClass From "/Game/00-Blueprints/Items/PortalGun/BP_PortalGunComponent.BP_PortalGunComponent_C")
  (Actor|DestroyActor))

(fn ConstructionScript
  (|CallParentFunction))