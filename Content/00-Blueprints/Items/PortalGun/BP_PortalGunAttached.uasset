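; Portal gun actor in its attached form, handling the gun's visuals, sounds and portal shots.
; On BeginPlay it caches the level's BP_Portal, tints its two point lights green and blue, and plays a timeline that rotates the crystals.
; Events swap the Portal_Color material and play a firing sound per portal.
; SendPortal spawns a BP_PortalBullet aimed at the target, passing it the placement data and portal reference.
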(event Custom|ChangeMaterial
  (params (FirstPortal :type Boolean))
  (Rendering|Material|SetMaterialbyName (Variables|Default|GetPortalGunMesh) "Portal_Color" (select FirstPortal (Variables|Default|GetMaterial1) (Variables|Default|GetMaterial2))))

(event Custom|PlayPortalSound
  (params (FirstPortal :type Boolean))
  (if FirstPortal
    (Audio|PlaySound2D (Variables|Default|GetSound1) 1.0 1.0 0.8 0 0)
    (else
      (Audio|PlaySound2D (Variables|Default|GetSound2) 1.0 1.0 0.3 0 0))))

(event Custom|SendPortal
  (params (First/Second :type Boolean) (StartLocation :type Vector) (EndLocation :type Vector) (Rotation :type Rotator) (WillPlacePortal :type Boolean))
  (bind _returnvalue (Math|Rotator|FindLookatRotation StartLocation EndLocation))
  (Game|SpawnActorfromClass "/Game/00-Blueprints/Items/PortalGun/BP_PortalBullet.BP_PortalBullet_C" (Math|Transform|MakeTransform (+ StartLocation (* (Math|Vector|GetForwardVector _returnvalue) 5e+01)) _returnvalue) "Undefined" "MultiplyWithRoot" 0 (select First/Second "/Game/00-Blueprints/Items/PortalGun/M_PortalBullet2.M_PortalBullet2" "/Game/00-Blueprints/Items/PortalGun/M_PortalBullet1.M_PortalBullet1") EndLocation Rotation First/Second (Variables|Default|GetPortal) WillPlacePortal 0))

(event EventBeginPlay
  (bind _returnvalue (Actor|GetActorOfClass "/Game/00-Blueprints/Items/PortalGun/BP_Portal.BP_Portal_C"))
  (Variables|Default|SetPortal _returnvalue)
  (Rendering|Components|Light|SetLightColor (Variables|Default|GetPointLight1) "(R=0.176471,G=1.000000,B=0.223529,A=1.000000)" true)
  (Rendering|Components|Light|SetLightColor (Variables|Default|GetPointLight) "(R=0.105882,G=0.454902,B=1.000000,A=1.000000)" true)
  (bind _newtrack_0 (Timeline|Timeline Play)
    (:Update
      (Transformation|SetRelativeRotation (Variables|Default|GetCrystals) (Math|Rotator|MakeRotator 0.0 _newtrack_0 0.0) false false))))

(event Collision|EventActorBeginOverlap
  (params (OtherActor :type Actor%20Object%20Reference)))

(event EventTick
  (params (DeltaSeconds :type Float%20%28single-precision%29)))

(fn ConstructionScript)