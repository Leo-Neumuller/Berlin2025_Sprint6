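; Crystal pedestal for the first enigma that accepts one crystal at a time and checks whether its type matches the pedestal's FeelingType.
; On sphere overlap it snaps the crystal into place, forces the player to ungrab, and turns its light green or red.
; Correct placements and removals adjust a shared counter on BP_FPSPlayer.
; When a placement brings that counter to three, the pedestal calls EnigmaIsValid.
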(event OnComponentBeginOverlap(Sphere)
  (params (OverlappedComponent :type Primitive%20Component%20Object%20Reference) (OtherActor :type Actor%20Object%20Reference) (OtherComp :type Primitive%20Component%20Object%20Reference) (OtherBodyIndex :type Integer) (bFromSweep :type Boolean) (SweepResult :type Hit%20Result%20Structure%20%28by%20ref%29))
  (Utilities|IsValid (Variables|Default|GetCrystalOnPiedestral)
    (:Is%20Not%20Valid
      (bind _asbp_item_crystals (Utilities|Casting|CastToBP_Item_Crystals OtherActor))
      (bind _output_get (Variables|Default|SetCrystalOnPiedestral _asbp_item_crystals))
      (Transformation|AttachComponentToComponent _output_get (Variables|Default|GetCrystalPos) "None" "SnapToTarget" "SnapToTarget" "KeepWorld" false)
      (Default|ForceUngrab (Variables|Default|GetPlayerRef))
      (if (Utilities|Enum|Equal(Enum) (Variables|/Game/00-Blueprints/Items/BP_Item_Crystals.BP_Item_Crystals_C|GetCrystalType _asbp_item_crystals) (Variables|01-FeelingType|GetFeelingType))
        (CallFunction|GoodCrystal)
        (Development|PrintString "GoodCrystal")
        (bind _result (Math|Integer|IncrementInt (Variables|/Game/00-Blueprints/Player/BP_FPSPlayer.BP_FPSPlayer_C|GetFirstEnigma_TotalValid (Variables|Default|GetPlayerRef)))
          (:%20%20
            (Development|PrintString (Utilities|String|Append "test: " (Utilities|String|ToString(Integer) _result)))
            (CallFunction|CheckifEnigmaIsOver)))
        (else
          (CallFunction|WrongCrystal)
          (Development|PrintString "WrongCrystal")))
      (Variables|Default|SetAlreadyHasACrystalOn true))))

(event OnComponentEndOverlap(Sphere)
  (params (OverlappedComponent :type Primitive%20Component%20Object%20Reference) (OtherActor :type Actor%20Object%20Reference) (OtherComp :type Primitive%20Component%20Object%20Reference) (OtherBodyIndex :type Integer))
  (if (Variables|Default|GetAlreadyHasACrystalOn)
    (if (== OtherActor (Variables|Default|GetCrystalOnPiedestral))
      (bind _asbp_item_crystals (Utilities|Casting|CastToBP_Item_Crystals OtherActor))
      (if (Utilities|Enum|Equal(Enum) (Variables|/Game/00-Blueprints/Items/BP_Item_Crystals.BP_Item_Crystals_C|GetCrystalType _asbp_item_crystals) (Variables|01-FeelingType|GetFeelingType))
        (bind _result (Math|Integer|DecrementInt (Variables|/Game/00-Blueprints/Player/BP_FPSPlayer.BP_FPSPlayer_C|GetFirstEnigma_TotalValid (Variables|Default|GetPlayerRef)))
          (:%20%20
            (Development|PrintString (Utilities|String|ToString(Integer) _result))
            (Rendering|Material|SetMaterial (Variables|Default|GetSM_Activated) 0 "/Engine/BasicShapes/BasicShapeMaterial.BasicShapeMaterial")))
        (else
          (Rendering|Components|Light|SetLightColor (Variables|Default|GetLightComponent0) "(R=1.000000,G=1.000000,B=1.000000,A=1.000000)" true)))
      (Variables|Default|SetAlreadyHasACrystalOn false)
      (Variables|Default|SetCrystalOnPiedestral 0))))

(event Custom|WrongCrystal
  (Rendering|Components|Light|SetLightColor (Variables|Default|GetLightComponent0) "(R=1.000000,G=0.102599,B=0.000000,A=1.000000)" true))

(event Custom|GoodCrystal
  (Rendering|Components|Light|SetLightColor (Variables|Default|GetLightComponent0) "(R=0.000000,G=1.000000,B=0.097419,A=1.000000)" true))

(event Custom|CheckIfEnigmaIsOver
  (if (== (Variables|/Game/00-Blueprints/Player/BP_FPSPlayer.BP_FPSPlayer_C|GetFirstEnigma_TotalValid (Variables|Default|GetPlayerRef)) 3)
    (Default|CallEnigmaIsValid)))

(event EventBeginPlay
  (bind _asbp_fpsplayer (Utilities|Casting|CastToBP_FPSPlayer (Game|GetPlayerCharacter 0)))
  (Variables|Default|SetPlayerRef _asbp_fpsplayer))

(fn ConstructionScript
  (|CallParentFunction))